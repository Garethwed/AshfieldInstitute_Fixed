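; Enemy pawn Blueprint that chases the third-person player when PawnSensing spots them.
; On sight it sets CanSeePlayer and runs AI MoveTo at the player, then clears the flag after a short delay and calls EnemyPatrolBetweenTargets.
; That event is empty, as the FlipFlop patrol between Target1 and Target2 is disconnected.
; A separate RunAtPlayer event moves toward the first player character found, but nothing here calls it.
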(event `self.PawnSensing.OnSeePawn`
  (params (Pawn :type "Pawn Object Reference"))
  (set `self.CanSeePlayer` true)
  (bind _asthird_person_character (cast `/Game/ThirdPersonBP/Blueprints/ThirdPersonCharacter` Pawn))
  (`|AIMoveTo` self (0.0 0.0 0.0) _asthird_person_character
    (:`OnSuccess`
      _)
    (:`OnFail`
      _))
  (`KismetSystemLibrary.Delay` 0.5)
  (set `self.CanSeePlayer` false)
  (`self.EnemyPatrolBetweenTargets`))

(event `self.ReceiveBeginPlay`)

(event `EnemyPatrolBetweenTargets`)

(event `RunAtPlayer`
  (bind _outactors (`GameplayStatics.GetAllActorsOfClass` "/Game/ThirdPersonBP/Blueprints/ThirdPersonCharacter.ThirdPersonCharacter_C"))
  (bind _asthird_person_character (cast `/Game/ThirdPersonBP/Blueprints/ThirdPersonCharacter` (`|GetArrayItem` _outactors)))
  (`|AIMoveTo` self (0.0 0.0 0.0) _asthird_person_character))

(fn `UserConstructionScript`)