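; Enemy pawn Blueprint that patrols between two target actors and chases the player when its PawnSensing component spots them.
; Patrol is a self-recalling event that alternates AIMoveTo between Target1 and Target2 via FlipFlop while CanSeePlayer is false.
; A sighting sets that flag and moves toward the ThirdPersonCharacter.
; When the chase move succeeds or fails, it waits briefly, clears the flag and resumes patrol.
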(event `self.PawnSensing.OnSeePawn`
  (params (Pawn :type "Pawn Object Reference"))
  (set `self.CanSeePlayer` true)
  (bind _asthird_person_character (cast `/Game/ThirdPersonBP/Blueprints/ThirdPersonCharacter` Pawn))
  (`|AIMoveTo` self (0.0 0.0 0.0) _asthird_person_character
    (:`OnSuccess`
      _)
    (:`OnFail`
      _))
  (`KismetSystemLibrary.Delay` 0.5)
  (set `self.CanSeePlayer` false)
  (`self.EnemyPatrolBetweenTargets`))

(event `self.ReceiveBeginPlay`
  (`self.EnemyPatrolBetweenTargets`))

(event `EnemyPatrolBetweenTargets`
  (if (not (`self.CanSeePlayer`))
    (`/Engine/EditorBlueprintResources/StandardMacros.FlipFlop`
      (:`A`
        (`|AIMoveTo` self (0.0 0.0 0.0) (`self.Target1`)
          (:`OnSuccess`
            _)
          (:`OnFail`
            _)))
      (:`B`
        (`|AIMoveTo` self (0.0 0.0 0.0) (`self.Target2`)
          (:`OnSuccess`
            _)
          (:`OnFail`
            _))))
    (`self.EnemyPatrolBetweenTargets`)))

(fn `UserConstructionScript`)