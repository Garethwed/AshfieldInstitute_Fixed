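; Pickupable torch item for the interaction system that the player can collect.
; On pickup it adds one unit of its item structure to the interacter's InventoryComponent, and only on success destroys itself.
; It then calls Pickuptorch on the ThirdPersonCharacter to trigger torch-specific handling.
; Using the item from the inventory does nothing and returns false.
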(event `/Game/InventorySystem/PickUpInterface.PickUp`
  (params (Interacter :type "Actor Object Reference"))
  (bind _success (`/Game/InventorySystem/InventoryComponent.AddToInventory` (`self.GetComponentByClass` Interacter "/Game/InventorySystem/InventoryComponent.InventoryComponent_C") (make `/Game/InventorySystem/SlotStructure` (`self.ItemStructure`) 1)))
  (if _success
    (`self.K2_DestroyActor`)
    (bind _asthird_person_character (cast `/Game/ThirdPersonBP/Blueprints/ThirdPersonCharacter` Interacter))
    (`/Game/ThirdPersonBP/Blueprints/ThirdPersonCharacter.pickuptorch` _asthird_person_character)))

(fn `Use Item`
  (returns (Succcess :type Boolean))
  (return false))

(fn `UserConstructionScript`
  (`parent.UserConstructionScript`))