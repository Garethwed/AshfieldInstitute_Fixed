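; BP_Key is a key pickup the player collects with the Interact input while inside its trigger box, which toggles input and prints a prompt.
; Pickup disables key collision and runs a looping timer that VInterps the actor toward the player character, then destroys it after a short delay.
; Setting PlayerHasKey1 is disconnected, so the pickup never records that the player has the key.
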(event `self.Trigger.OnComponentBeginOverlap`
  (params (OverlappedComponent :type "PrimitiveComponent Object Reference") (OtherActor :type "Actor Object Reference") (OtherComp :type "PrimitiveComponent Object Reference") (OtherBodyIndex :type Integer) (bFromSweep :type Boolean) (SweepResult :type "HitResult Structure (by ref)"))
  ;[1 1 1] Triggerbox
  (`self.EnableInput` (`GameplayStatics.GetPlayerController` 0))
  (`KismetSystemLibrary.PrintText` "(E) Key"))

(event `self.Trigger.OnComponentEndOverlap`
  (params (OverlappedComponent :type "PrimitiveComponent Object Reference") (OtherActor :type "Actor Object Reference") (OtherComp :type "PrimitiveComponent Object Reference") (OtherBodyIndex :type Integer))
  ;[1 1 1] Triggerbox
  (`self.DisableInput` (`GameplayStatics.GetPlayerController` 0)))

(event `InputAction|Interact`
  (params (Key :type "Key Structure"))
  (:`Pressed`
    (`self.Key_movement`)))

(event `Key_movement`
  ;[1 1 1] Variable setup
  (`KismetSystemLibrary.K2_SetTimerDelegate` (delegate `Movement`) 0.01 true)
  (`PrimitiveComponent.SetCollisionEnabled` (`self.Key`) "NoCollision")
  (`KismetSystemLibrary.Delay` 0.5)
  (`self.K2_DestroyActor`)
  (cast `/Game/ThirdPersonBP/Blueprints/ThirdPersonCharacter` (`GameplayStatics.GetPlayerCharacter` 0)))

(event `Movement`
  (bind _defaultsceneroot (`self.DefaultSceneRoot`))
  ;[1 1 1] Pick up movement
  (bind _asthird_person_character (cast `/Game/ThirdPersonBP/Blueprints/ThirdPersonCharacter` (`GameplayStatics.GetPlayerCharacter` 0)))
  (`SceneComponent.K2_SetWorldLocation` _defaultsceneroot (`KismetMathLibrary.VInterpTo` (`SceneComponent.K2_GetComponentLocation` _defaultsceneroot) (`self.K2_GetActorLocation` _asthird_person_character) (`GameplayStatics.GetWorldDeltaSeconds`) 3.0) false false))

(fn `UserConstructionScript`)