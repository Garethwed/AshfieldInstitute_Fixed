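; Automatic door actor, apparently the right-hand variant, that swings open and closed around yaw based on player proximity.
; Trigger begin and end overlaps play the Rotation timeline if player 0 is within 300 units, otherwise reverse it.
; Timeline updates combine the yaw with the rotation saved at BeginPlay.
; Each update also rechecks distance, a bug fix letting the door change direction mid-rotation.
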(event `self.Trigger.OnComponentBeginOverlap`
  (params (OverlappedComponent :type "PrimitiveComponent Object Reference") (OtherActor :type "Actor Object Reference") (OtherComp :type "PrimitiveComponent Object Reference") (OtherBodyIndex :type Integer) (bFromSweep :type Boolean) (SweepResult :type "HitResult Structure (by ref)"))
  ;[1 1 1] Triggerbox
  ;[1 1 1] Configure rotator
  (if (>= (`self.GetDistanceTo` (`GameplayStatics.GetPlayerCharacter` 0)) 300.0) :!label _label
    (bind (_direction _door_rotation) (`Timeline|Rotation` :!via `Reverse` :!label _label_2)
      (:`Update`
        (`self.K2_SetActorRelativeRotation` (`KismetMathLibrary.ComposeRotators` (`KismetMathLibrary.MakeRotator` 0.0 0.0 _door_rotation) (`self.Porte_ini`)))
        ;;[1 1 1] BugFixWhileItRotates
        (if (>= (`self.GetDistanceTo` (`GameplayStatics.GetPlayerCharacter` 0)) 300.0)
          (goto _label_2 :!via `Reverse`)
          (else
            (goto _label_2)))))
    (else
      (goto _label_2))))

(event `self.Trigger.OnComponentEndOverlap`
  (params (OverlappedComponent :type "PrimitiveComponent Object Reference") (OtherActor :type "Actor Object Reference") (OtherComp :type "PrimitiveComponent Object Reference") (OtherBodyIndex :type Integer))
  ;[1 1 1] Triggerbox
  (goto _label))

(event `self.ReceiveBeginPlay`
  ;[1 1 1] Init
  (set `self.Porte_ini` (`self.K2_GetActorRotation`)))

(fn `UserConstructionScript`)