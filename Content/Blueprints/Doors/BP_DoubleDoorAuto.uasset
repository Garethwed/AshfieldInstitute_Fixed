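; Automatic double door Blueprint that swings both leaves open when something overlaps its Trigger volume and closes them when the overlap ends.
; Separate left and right timelines drive yaw offsets, playing on begin overlap and reversing on end overlap.
; Each offset is combined with that door's relative rotation cached at BeginPlay, so the swing is relative to its initial placed orientation.
; The overlapping actor is not filtered.
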(event `self.Trigger.OnComponentBeginOverlap`
  (params (OverlappedComponent :type "PrimitiveComponent Object Reference") (OtherActor :type "Actor Object Reference") (OtherComp :type "PrimitiveComponent Object Reference") (OtherBodyIndex :type Integer) (bFromSweep :type Boolean) (SweepResult :type "HitResult Structure (by ref)"))
  ;[1 1 1] Triggerbox
  (`|ExecutionSequence`
    (:`then_0`
      ;[1 1 1] RightDoor
      (bind (_direction _door_rotation) (`Timeline|DoorRightRotation` :!label _label)
        (:`Update`
          (`SceneComponent.K2_SetRelativeRotation` (`self.DoorRight`) (`KismetMathLibrary.ComposeRotators` (`KismetMathLibrary.MakeRotator` 0.0 0.0 _door_rotation) (`self.Porte_iniRight`)) false false))))
    (:`then_1`
      ;[1 1 1] LeftDoor
      (bind (_direction_2 _door_rotation_2) (`Timeline|DoorLeftRotation` :!label _label_2)
        (:`Update`
          (`SceneComponent.K2_SetRelativeRotation` (`self.DoorLeft`) (`KismetMathLibrary.ComposeRotators` (`KismetMathLibrary.MakeRotator` 0.0 0.0 _door_rotation_2) (`self.Porte_iniLeft`)) false false))))))

(event `self.Trigger.OnComponentEndOverlap`
  (params (OverlappedComponent :type "PrimitiveComponent Object Reference") (OtherActor :type "Actor Object Reference") (OtherComp :type "PrimitiveComponent Object Reference") (OtherBodyIndex :type Integer))
  ;[1 1 1] Triggerbox
  (`|ExecutionSequence`
    (:`then_0`
      (goto _label :!via `Reverse`))
    (:`then_1`
      (goto _label_2 :!via `Reverse`))))

(event `self.ReceiveBeginPlay`
  ;[1 1 1] Init
  (set `self.Porte_iniLeft` (`SceneComponent.RelativeRotation` (`self.DoorLeft`)))
  (set `self.Porte_iniRight` (`SceneComponent.RelativeRotation` (`self.DoorRight`))))

(fn `UserConstructionScript`)