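; AI controller for the ZombieTut enemy, linking its perception and behavior tree.
; On possessing a ZombieTut, it caches the pawn and runs the TutTree behavior tree.
; AI Perception updates on a ThirdPersonCharacter write the sensed result to the CanSee blackboard key.
; Walk and Run events forward to the cached zombie's matching functions.
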(event `self.AIPerception.OnTargetPerceptionUpdated`
  (params (Actor :type "Actor Object Reference") (Stimulus :type "AIStimulus Structure"))
  (cast `/Game/ThirdPersonBP/Blueprints/ThirdPersonCharacter` Actor)
  (`BlackboardComponent.SetValueAsBool` (`AIBlueprintHelperLibrary.GetBlackboard` null) "CanSee" (`.bSuccessfullySensed` (break `AIStimulus` Stimulus))))

(event `Walk`
  (`/Game/Blueprints/ChaseRoamEnemy/ZombieTut.Walk` (`self.Zombie`)))

(event `Run`
  (`/Game/Blueprints/ChaseRoamEnemy/ZombieTut.Run` (`self.Zombie`)))

(event `self.OnPossess`
  (params (PossessedPawn :type "Pawn Object Reference"))
  (bind _aszombie_tut (cast `/Game/Blueprints/ChaseRoamEnemy/ZombieTut` PossessedPawn))
  (set `self.Zombie` _aszombie_tut)
  (`self.RunBehaviorTree` "/Game/Blueprints/ChaseRoamEnemy/TutTree.TutTree"))

(fn `UserConstructionScript`)