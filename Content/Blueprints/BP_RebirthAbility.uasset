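; Rebirth ability actor that temporarily lifts enemies touching its hitbox into the air, then drops them back down after a fixed delay.
; On overlap, a ZombieTut is teleported straight up from its own position, while an EnemyPath is teleported above the ability actor's position.
; Each branch then waits and teleports that enemy down by the same height.
; An unwired branch for the old BasicAICharacter enemy remains unused.
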(event `self.Hitbox.OnComponentBeginOverlap`
  (params (OverlappedComponent :type "PrimitiveComponent Object Reference") (OtherActor :type "Actor Object Reference") (OtherComp :type "PrimitiveComponent Object Reference") (OtherBodyIndex :type Integer) (bFromSweep :type Boolean) (SweepResult :type "HitResult Structure (by ref)"))
  (bind (_returnvalue_x _returnvalue_y _returnvalue_z) (`KismetMathLibrary.BreakVector` (`self.K2_GetActorLocation`)))
  (bind _aszombie_tut (cast `/Game/Blueprints/ChaseRoamEnemy/ZombieTut` OtherActor)
    (:`then`
      (bind (_returnvalue_x_2 _returnvalue_y_2 _returnvalue_z_2) (`KismetMathLibrary.BreakVector` (`self.K2_GetActorLocation` _aszombie_tut)))
      (`self.K2_TeleportTo` :`self` _aszombie_tut :`DestLocation` (`KismetMathLibrary.MakeVector` _returnvalue_x_2 _returnvalue_y_2 (+ 600.0 _returnvalue_z_2)))
      (`KismetSystemLibrary.Delay` 15.0)
      (bind (_returnvalue_x_3 _returnvalue_y_3 _returnvalue_z_3) (`KismetMathLibrary.BreakVector` (`self.K2_GetActorLocation` _aszombie_tut)))
      (`self.K2_TeleportTo` :`self` _aszombie_tut :`DestLocation` (`KismetMathLibrary.MakeVector` _returnvalue_x_3 _returnvalue_y_3 (- _returnvalue_z_3 600.0))))
    (:`CastFailed`
      (bind _asenemy_path (cast `/Game/Blueprints/EnemyWithTarget/EnemyPath` OtherActor))
      (`self.K2_TeleportTo` :`self` _asenemy_path :`DestLocation` (`KismetMathLibrary.MakeVector` _returnvalue_x _returnvalue_y (+ 600.0 _returnvalue_z)))
      (`KismetSystemLibrary.Delay` 15.0)
      (bind (_returnvalue_x_4 _returnvalue_y_4 _returnvalue_z_4) (`KismetMathLibrary.BreakVector` (`self.K2_GetActorLocation` _asenemy_path)))
      (`self.K2_TeleportTo` :`self` _asenemy_path :`DestLocation` (`KismetMathLibrary.MakeVector` _returnvalue_x_4 _returnvalue_y_4 (- _returnvalue_z_4 600.0))))))

(fn `UserConstructionScript`)